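; BP_N_Block is a block actor that suppresses other blocks overlapping its Box component.
; On begin overlap it ignores itself and actors tagged "Sequence", and acts only on actors tagged "Block".
; Each match is added to the NOverlapedActors collection, then hidden and stripped of collision rather than destroyed.
; Nothing in this Blueprint restores or reads back the stored actors.
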(event `self.Box.OnComponentBeginOverlap`
  (params (OverlappedComponent :type "PrimitiveComponent Object Reference") (OtherActor :type "Actor Object Reference") (OtherComp :type "PrimitiveComponent Object Reference") (OtherBodyIndex :type Integer) (bFromSweep :type Boolean) (SweepResult :type "HitResult Structure (by ref)"))
  (if (`self.ActorHasTag` OtherActor "Sequence")
    _
    (elif (and (!= OtherActor self) (`self.ActorHasTag` OtherActor "Block"))
      (`KismetArrayLibrary.Array_Add` (`self.N_OverlapedActors`) OtherActor)
      (`self.SetActorHiddenInGame` OtherActor true)
      (`self.SetActorEnableCollision` OtherActor false))))

(fn `UserConstructionScript`)