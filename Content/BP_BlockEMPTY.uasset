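; BP_BlockEMPTY is a block Blueprint with a Widget and a BlockManager reference, but no active logic in its graphs.
; BeginPlay and the construction script are empty.
; A disconnected, never-run branch would rotate the Widget to match BlockManager's arrow direction for Arrow blocks, and hide it for other types.
; That branch compares enums by converting them to strings.
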(event `self.ReceiveBeginPlay`)

(fn `UserConstructionScript`)