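; Enemy actor that, while killable, is replaced by a block when the player character hits it.
; A hit on its TriggerInvincible component checks for the third-person character, the CanKill flag and a valid BlockToSpawn reference.
; It then spawns a new actor of that block's class, moves it slightly below the enemy's position and destroys itself.
; Only hit response is implemented, with leftover debug prints and no movement or AI logic.
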(event `self.ReceiveBeginPlay`)

(event `self.TriggerInvincible.OnComponentHit`
  (params (HitComponent :type "PrimitiveComponent Object Reference") (OtherActor :type "Actor Object Reference") (OtherComp :type "PrimitiveComponent Object Reference") (NormalImpulse :type "Vector Structure") (Hit :type "HitResult Structure (by ref)"))
  (bind _blocktospawn (`self.BlockToSpawn`))
  (cast `/Game/ThirdPerson/Blueprints/BP_ThirdPersonCharacter` OtherActor
    (:`then`
      (if (`self.canKill`)
        (`/Engine/EditorBlueprintResources/StandardMacros.IsValid` _blocktospawn
          (:`Is Valid`
            (bind _returnvalue (`|SpawnActorFromClass` (`GameplayStatics.GetObjectClass` _blocktospawn) (`self.GetTransform` _blocktospawn) "Undefined" "OverrideRootScale" null null))
            (`self.K2_SetActorLocation` _returnvalue (- (`self.K2_GetActorLocation`) (0.0 0.0 60.0)) false false)
            (`self.K2_DestroyActor`)
            (`KismetSystemLibrary.PrintString` "Hello")))))
    (:`CastFailed`
      (`KismetSystemLibrary.PrintString` "Hello"))))

(fn `UserConstructionScript`)