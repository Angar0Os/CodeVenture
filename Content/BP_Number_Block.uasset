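; Number block actor that displays its Number through a widget and absorbs other blocks that overlap it.
; Each Tick, unless the player character's Actor reference points to this block, it traces along its local down axis and snaps to the hit location.
; On box overlap, other "Block"-tagged actors without a "Sequence" tag are added to NumberOverlapedActors, hidden and stripped of collision.
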(event `self.ReceiveTick`
  (params (DeltaSeconds :type "Float (single-precision)"))
  (bind _returnvalue (`self.K2_GetActorLocation`))
  (bind _asbp_third_person_character (cast `/Game/ThirdPerson/Blueprints/BP_ThirdPersonCharacter` (`GameplayStatics.GetPlayerCharacter` 0)))
  (if (not (== (`/Game/ThirdPerson/Blueprints/BP_ThirdPersonCharacter.actor` _asbp_third_person_character) self))
    (bind _outhit (`KismetSystemLibrary.LineTraceSingle` _returnvalue (+ _returnvalue (* (`KismetMathLibrary.GetUpVector` (`self.K2_GetActorRotation`)) -100000.0)) "TraceTypeQuery1"))
    (bind (_bblockinghit _binitialoverlap _time _distance _location) (`GameplayStatics.BreakHitResult` _outhit))
    (if _bblockinghit
      (bind _output_get (set `self.spawnLocation` _location))
      (`self.K2_SetActorLocation` _output_get))))

(event `self.ReceiveBeginPlay`
  (bind _asnumber (cast `/Game/Assets/UI/Number` (`WidgetComponent.GetWidget` (`self.Widget`))))
  (set `/Game/Assets/UI/Number.txtNb` (`self.Number`) _asnumber))

(event `self.Box.OnComponentBeginOverlap`
  (params (OverlappedComponent :type "PrimitiveComponent Object Reference") (OtherActor :type "Actor Object Reference") (OtherComp :type "PrimitiveComponent Object Reference") (OtherBodyIndex :type Integer) (bFromSweep :type Boolean) (SweepResult :type "HitResult Structure (by ref)"))
  (if (`self.ActorHasTag` OtherActor "Sequence")
    _
    (elif (and (!= OtherActor self) (`self.ActorHasTag` OtherActor "Block"))
      (`KismetArrayLibrary.Array_Add` (`self.Number_OverlapedActors`) OtherActor)
      (`self.SetActorHiddenInGame` OtherActor true)
      (`self.SetActorEnableCollision` OtherActor false))))

(fn `UserConstructionScript`)